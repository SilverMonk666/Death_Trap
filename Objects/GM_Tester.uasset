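; GM_Tester is a Game Mode that restores the key card when a player restarts.
; On BeginPlay it records the transform of the first BP_KeyCard found in the level and sets a GameStarted flag.
; Once that flag is set, OnRestartPlayer checks for an existing key card and spawns a new one at the saved transform if none is valid.
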(event `self.ReceiveBeginPlay`
  (bind _outactors (`GameplayStatics.GetAllActorsOfClass` "/Game/Objects/Blueprints/BP_Interacts/BP_KeyCard.BP_KeyCard_C"))
  (set `self.Transform` (`self.GetTransform` (`|GetArrayItem` _outactors)))
  (set `self.GameStarted` true))

(event `self.K2_OnRestartPlayer`
  (params (NewPlayer :type "Controller Object Reference"))
  (if (`self.GameStarted`)
    (bind _outactors (`GameplayStatics.GetAllActorsOfClass` "/Game/Objects/Blueprints/BP_Interacts/BP_KeyCard.BP_KeyCard_C"))
    (`/Engine/EditorBlueprintResources/StandardMacros.IsValid` (`|GetArrayItem` _outactors)
      (:`Is Not Valid`
        (`|SpawnActorFromClass` "/Game/Objects/Blueprints/BP_Interacts/BP_KeyCard.BP_KeyCard_C" (`self.Transform`) "Undefined" "OverrideRootScale" null null)))))

(fn `UserConstructionScript`)