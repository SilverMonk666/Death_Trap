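; Moving platform actor whose Cube component shuttles back and forth along its relative X axis in an endless loop.
; Tick enters a DoOnce that starts a latent chain: pause, eased MoveComponentTo forward by a fixed offset, pause, then eased move back by the same offset.
; The DoOnce resets when the chain finishes, so a later Tick starts the next cycle.
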(event `self.ReceiveTick`
  (params (DeltaSeconds :type "Float (single-precision)"))
  (bind _cube (`self.Cube`))
  (bind _cube_2 (`self.Cube`))
  (bind (_relativelocation_x _relativelocation_y _relativelocation_z) (`KismetMathLibrary.BreakVector` (`SceneComponent.RelativeLocation` _cube_2)))
  (bind (_relativelocation_x_2 _relativelocation_y_2 _relativelocation_z_2) (`KismetMathLibrary.BreakVector` (`SceneComponent.RelativeLocation` _cube)))
  (`/Engine/EditorBlueprintResources/StandardMacros.DoOnce` false :!label _label
    (:`Completed`
      (`KismetSystemLibrary.Delay` 1.0)
      (`KismetSystemLibrary.MoveComponentTo` _cube (`KismetMathLibrary.MakeVector` (+ _relativelocation_x_2 500.0) _relativelocation_y_2 _relativelocation_z_2) (`SceneComponent.RelativeRotation` _cube) true true 1.0)
      (`KismetSystemLibrary.Delay` 1.0)
      (`KismetSystemLibrary.MoveComponentTo` _cube_2 (`KismetMathLibrary.MakeVector` (- _relativelocation_x 500.0) _relativelocation_y _relativelocation_z) (`SceneComponent.RelativeRotation` _cube_2) true true 1.0)
      (goto _label :!via `Reset`))))

(fn `UserConstructionScript`)