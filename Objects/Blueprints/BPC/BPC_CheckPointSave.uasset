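; Checkpoint respawn component that resets the level and restarts the first player at an interactive checkpoint.
; ResSpawn scans all BP_InteractiveCheckPoint actors for those whose OnOffState is the enum's first entry and stores each match in CheckPoints.
; Each match triggers the GameMode's ResetLevel and RestartPlayerAtPlayerStart, as the loop has no break.
; The component's own event graph never runs ResSpawn.
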(fn `ResSpawn`
  (bind _returnvalue (`GameplayStatics.GetGameMode`))
  (bind _outactors (`GameplayStatics.GetAllActorsOfClass` "/Game/Objects/Blueprints/BP_InteractiveCheckPoint.BP_InteractiveCheckPoint_C"))
  (for _array_element _outactors
    (if (`|EnumEquality` (`/Game/Objects/Blueprints/BP_InteractiveCheckPoint.OnOffState` _array_element) "NewEnumerator0")
      (bind _output_get (set `self.CheckPoints` _array_element))
      (`GameModeBase.ResetLevel` _returnvalue)
      (`GameModeBase.RestartPlayerAtPlayerStart` _returnvalue (`GameplayStatics.GetPlayerController` 0) _output_get))))