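; BP_KeyCard is an interactable keycard pickup that grants the player KeyCard01.
; Interact fires Pickup, which ignores Pawn and Camera collision on its THing component, disables Trigger physics and attaches it to a socket component.
; After a brief delay it sets KeyCard01 on the PhasePlayerCharacter and destroys itself.
; DropItems calls an empty DropItem event, with detach and held-item logic left disconnected.
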(event `Pickup`
  (params (Socket :type "SceneComponent Object Reference") (Actor :type "Actor Object Reference"))
  (bind _thing (`self.THing`))
  (`PrimitiveComponent.SetCollisionResponseToChannel` _thing "ECC_Pawn" "ECR_Ignore")
  (`PrimitiveComponent.SetCollisionResponseToChannel` _thing "ECC_Camera" "ECR_Ignore")
  (`PrimitiveComponent.SetSimulatePhysics` (`self.Trigger`) false)
  (`self.K2_AttachToComponent` Socket "None" "SnapToTarget" "SnapToTarget" "KeepRelative")
  (`KismetSystemLibrary.PrintString` "Worked")
  (bind _asphase_player_character (cast `/Game/BlueprintCharacters/PhasePlayerCharacter` (`GameplayStatics.GetPlayerCharacter` 0)))
  (`KismetSystemLibrary.Delay` 0.2)
  (set `/Game/BlueprintCharacters/PhasePlayerCharacter.KeyCard01` true _asphase_player_character)
  (`self.K2_DestroyActor`))

(event `DropItem`)

(fn `DropItems`
  (returns (Val :type Boolean))
  (`self.DropItem`)
  (return false))

(fn `Interact`
  (params (TargetPoint :type "SceneComponent Object Reference") (Actor :type "Actor Object Reference"))
  (returns (Val :type Boolean))
  (`self.Pickup` null)
  (return false))

(fn `UserConstructionScript`
  (`parent.UserConstructionScript`))