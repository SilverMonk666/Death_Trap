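; Rising water hazard that sends the player back to a checkpoint on contact.
; Tick re-issues MoveComponentTo toward a point slightly above the current height, so the Water component creeps upward continuously.
; A Character overlapping the Trigger calls ResSpawn on BPCCheckPointSave with the player start.
; OnReset snaps the water back to its stored restart location.
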(event `self.K2_OnReset`
  (bind _waterrestartlocation_location (`KismetMathLibrary.BreakTransform` (`self.WaterRestartLocation`)))
  (`SceneComponent.K2_SetWorldLocation` (`self.Water`) _waterrestartlocation_location false false))

(event `self.ReceiveTick`
  (params (DeltaSeconds :type "Float (single-precision)"))
  (bind _water (`self.Water`))
  (bind (_relativelocation_x _relativelocation_y _relativelocation_z) (`KismetMathLibrary.BreakVector` (`SceneComponent.RelativeLocation` _water)))
  (`KismetSystemLibrary.MoveComponentTo` _water (`KismetMathLibrary.MakeVector` _relativelocation_x _relativelocation_y (+ _relativelocation_z 10.0)) (`SceneComponent.RelativeRotation` _water) false false 10.0))

(event `self.Trigger.OnComponentBeginOverlap`
  (params (OverlappedComponent :type "PrimitiveComponent Object Reference") (OtherActor :type "Actor Object Reference") (OtherComp :type "PrimitiveComponent Object Reference") (OtherBodyIndex :type Integer) (bFromSweep :type Boolean) (SweepResult :type "HitResult Structure (by ref)"))
  (cast `Character` OtherActor)
  (`/Game/Objects/Blueprints/BPC/BPC_CheckPointSave.ResSpawn` (`self.BPC_CheckPointSave`) (`self.ThePlayerStart`)))

(fn `UserConstructionScript`)