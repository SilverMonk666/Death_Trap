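; Keycard terminal interactable that sets linked moving platforms in motion when the player holds the first keycard.
; Its Interact function calls the Unlock event and always returns false, ignoring the passed target point and actor.
; Unlock casts player character 0 to PhasePlayerCharacter, checks its KeyCard01 flag, and calls MovePlatform on every entry in the MovingPlatform array.
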(event `Unlock`
  (bind _asphase_player_character (cast `/Game/BlueprintCharacters/PhasePlayerCharacter` (`GameplayStatics.GetPlayerCharacter` 0)))
  (if (`/Game/BlueprintCharacters/PhasePlayerCharacter.KeyCard01` _asphase_player_character)
    (for _array_element (`self.MovingPlatform`)
      (`/Game/Objects/Blueprints/BP_MovingPlatform.MovePlatform` _array_element))))

(fn `Interact`
  (params (TargetPoint :type "SceneComponent Object Reference") (Actor :type "Actor Object Reference"))
  (returns (Val :type Boolean))
  (`self.Unlock`)
  (return false))

(fn `UserConstructionScript`
  (`parent.UserConstructionScript`))