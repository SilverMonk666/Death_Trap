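; BoxCutter is a physics cube that splits into eight smaller pieces when a ThirdPersonCharacter overlaps it while casting an ability.
; Cut spawns pieces at eight arrow transforms with halved scale, copies the cube's linear and angular velocity, then destroys the original.
; Splitting is recursive: above MaxcutLevel scale the pieces are new BoxCutters with an added location-based impulse; otherwise they are SmallCubes without one.
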(event `self.Cube.OnComponentBeginOverlap`
  (params (OverlappedComponent :type "PrimitiveComponent Object Reference") (OtherActor :type "Actor Object Reference") (OtherComp :type "PrimitiveComponent Object Reference") (OtherBodyIndex :type Integer) (bFromSweep :type Boolean) (SweepResult :type "HitResult Structure (by ref)"))
  (bind _asthird_person_character (cast `/Game/ThirdPersonBP/Blueprints/ThirdPersonCharacter` OtherActor))
  (if (`/Game/ThirdPersonBP/Blueprints/ThirdPersonCharacter.CastingAbility` _asthird_person_character)
    (`self.Cut`)))

(event `self.Cube.OnComponentEndOverlap`
  (params (OverlappedComponent :type "PrimitiveComponent Object Reference") (OtherActor :type "Actor Object Reference") (OtherComp :type "PrimitiveComponent Object Reference") (OtherBodyIndex :type Integer))
  (cast `/Game/ThirdPersonBP/Blueprints/ThirdPersonCharacter` OtherActor))

(fn `Cut`
  (bind _cube (`self.Cube`))
  (bind _cube_2 (`self.Cube`))
  (bind _returnvalue_x (`KismetMathLibrary.BreakVector` (`SceneComponent.K2_GetComponentScale` (`self.Cube`))))
  (if (> _returnvalue_x (`self.MaxcutLevel`))
    (bind _returnvalue (`PrimitiveComponent.GetPhysicsAngularVelocityInDegrees` _cube "None"))
    (set `self.AngularVilocity` _returnvalue)
    (bind _returnvalue_2 (`PrimitiveComponent.GetPhysicsLinearVelocity` _cube "None"))
    (set `self.LinearVilocityt` _returnvalue_2)
    (for _array_element (`self.Position`)
      (bind (_returnvalue_location _returnvalue_rotation _returnvalue_scale) (`KismetMathLibrary.BreakTransform` (`SceneComponent.K2_GetComponentToWorld` _array_element)))
      (bind _returnvalue_3 (`|SpawnActorFromClass` "BoxCutter_C" (`KismetMathLibrary.MakeTransform` _returnvalue_location _returnvalue_rotation (/ _returnvalue_scale 2.0)) "Undefined" "OverrideRootScale" null null))
      (bind _cube_3 (`/Objects/Blueprints/BoxCutter.Cube` _returnvalue_3))
      (`PrimitiveComponent.SetPhysicsLinearVelocity` _cube_3 (`self.LinearVilocityt`) false "None")
      (`PrimitiveComponent.SetPhysicsAngularVelocityInDegrees` _cube_3 (`self.AngularVilocity`) false "None")
      (`PrimitiveComponent.AddImpulseAtLocation` (`/Objects/Blueprints/BoxCutter.Cube` _returnvalue_3) (* (`self.K2_GetActorLocation` _returnvalue_3) 100.0) (`SceneComponent.RelativeLocation` (`self.w`)) "None"))
    (`self.K2_DestroyActor`)
    (else
      (bind _returnvalue_4 (`PrimitiveComponent.GetPhysicsAngularVelocityInDegrees` _cube_2 "None"))
      (set `self.AngularVilocity` _returnvalue_4)
      (bind _returnvalue_5 (`PrimitiveComponent.GetPhysicsLinearVelocity` _cube_2 "None"))
      (set `self.LinearVilocityt` _returnvalue_5)
      (for _array_element_2 (`self.Position`)
        (bind (_returnvalue_location_2 _returnvalue_rotation_2 _returnvalue_scale_2) (`KismetMathLibrary.BreakTransform` (`SceneComponent.K2_GetComponentToWorld` _array_element_2)))
        (bind _returnvalue_6 (`|SpawnActorFromClass` "/Game/Objects/Blueprints/SmallCube.SmallCube_C" (`KismetMathLibrary.MakeTransform` _returnvalue_location_2 _returnvalue_rotation_2 (/ _returnvalue_scale_2 2.0)) "Undefined" "OverrideRootScale" null null))
        (bind _cube_4 (`/Game/Objects/Blueprints/SmallCube.Cube` _returnvalue_6))
        (`PrimitiveComponent.SetPhysicsLinearVelocity` _cube_4 (`self.LinearVilocityt`) false "None")
        (`PrimitiveComponent.SetPhysicsAngularVelocityInDegrees` _cube_4 (`self.AngularVilocity`) false "None"))
      (`self.K2_DestroyActor`))))

(fn `UserConstructionScript`
  (set `self.Position` (`|MakeArray` (`self.Arrow1`) (`self.Arrow2`) (`self.Arrow3`) (`self.Arrow4`) (`self.Arrow5`) (`self.Arrow6`) (`self.Arrow7`) (`self.Arrow`))))