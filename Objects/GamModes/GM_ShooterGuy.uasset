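; Game mode for a shooter that adds a keycard widget to the viewport and runs a countdown game timer.
; On player restart it restores inventory, held item and keycard from stored references, and resets the timer if it has expired.
; Tick uses a Delay to count down each second, printing the time on screen.
; At zero it prints a game-over message and switches every interactive checkpoint off.
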(event `self.ReceiveBeginPlay`
  ;[1 1 1] Begin Play create Keycard widget
  (bind _returnvalue (`|CreateWidget` "/Game/Objects/Widgets/Keycard_Widgets.Keycard_Widgets_C" (`GameplayStatics.GetPlayerController` 0)))
  (`UserWidget.AddToViewport` _returnvalue 0))

(event `self.K2_OnRestartPlayer`
  (params (NewPlayer :type "Controller Object Reference"))
  (bind _inventoryref (`self.InventoryRef`))
  ;[1 1 1] Setting All variables back on respawning Playr
  (`/Engine/EditorBlueprintResources/StandardMacros.IsValid` NewPlayer
    (:`Is Valid`
      (bind _asphase_player_character (cast `/Game/BlueprintCharacters/PhasePlayerCharacter` (`GameplayStatics.GetPlayerCharacter` 0)))
      (set `/Game/BlueprintCharacters/PhasePlayerCharacter.Inventory` _inventoryref _asphase_player_character)
      (bind _output_get (set `self.InHand` (`|GetArrayItem` _inventoryref)))
      (set `/Game/BlueprintCharacters/PhasePlayerCharacter.ItemInHand` _output_get _asphase_player_character)
      (set `/Game/BlueprintCharacters/PhasePlayerCharacter.KeyCard01` (`self.Keycard01Ref`) _asphase_player_character)
      (if (`self.TimerDone?`)
        (set `self.TimerDone?` false)
        (set `self.Minutes` 0)
        (set `self.Seconds` 20)))))

(event `self.ReceiveTick`
  (params (DeltaSeconds :type "Float (single-precision)"))
  ;[1 1 1] GameTimer
  (if (not (`self.TimerDone?`))
    (`KismetSystemLibrary.Delay` 1.0)
    (set `self.Seconds` (- (`self.Seconds`) 1))
    (if (< (`self.Seconds`) 0)
      (set `self.Minutes` (- (`self.Minutes`) 1))
      (set `self.Seconds` 59))
    (`KismetSystemLibrary.PrintString` (`KismetStringLibrary.Concat_StrStr` (`KismetStringLibrary.Conv_IntToString` (`self.Minutes`)) ":" (`KismetStringLibrary.Conv_IntToString` (`self.Seconds`))))
    (if (== (`self.Seconds`) 0)
      (if (== (`self.Minutes`) 0)
        (set `self.TimerDone?` true)
        (`KismetSystemLibrary.PrintString` "GameOver  \nYou Ran Out Of Time")
        ;[1 1 1] Update all Check points to Off when Timer Runs out
        (bind _outactors (`GameplayStatics.GetAllActorsOfClass` "/Game/Objects/Blueprints/BP_InteractiveCheckPoint.BP_InteractiveCheckPoint_C"))
        (for _array_element _outactors
          (set `/Game/Objects/Blueprints/BP_InteractiveCheckPoint.OnOffState` "NewEnumerator1" _array_element))))))

(fn `UserConstructionScript`)